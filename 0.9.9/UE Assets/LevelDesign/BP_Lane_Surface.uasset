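; Lane surface actor that builds a flat-segmented strip mesh along a spline in the construction script, with no active runtime logic.
; Each spline segment becomes a four-vertex procedural mesh section with the assigned material, using straight edges between points.
; Corners are mitered by intersecting the width-offset lines of adjacent segments in 2D, with fallbacks for the first point and parallel lines.
; An optional Z override replaces vertex heights.
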(event EventBeginPlay)

(event Collision|EventActorBeginOverlap
  (params (OtherActor :type Actor%20Object%20Reference)))

(event EventTick
  (params (DeltaSeconds :type Float%20%28single-precision%29)))

(fn ConstructionScript
  (bind _returnvalue (AddComponent|AddProceduralMeshComponent false))
  (Variables|Default|Setmesh _returnvalue)
  (for _index (range 0 (Class|SplineComponent|GetNumberOfSplineSegments (Variables|Default|GetSpline)))
    (bind (_point_1 _point_2) (Utilities|GetCornersatSplinePoint _index)
      (:Exec_out
        (bind (_point_1_2 _point_2_2) (Utilities|GetCornersatSplinePoint (+ _index 1))
          (:Exec_out
            (Class|ProceduralMeshComponent|CreateMeshSectionLinearColor (Variables|Default|Getmesh) _index (Utilities|Array|MakeArray (Utilities|DoZOverride _point_1) (Utilities|DoZOverride _point_2) (Utilities|DoZOverride _point_1_2) (Utilities|DoZOverride _point_2_2)) (Variables|Default|Gettriangle_indices) 0 0 0 0 0 0 0 false)
            (Rendering|Material|SetMaterial (Variables|Default|Getmesh) _index (Variables|Default|Getmaterial))))))))

(fn LineIntersection
  (params (a_point :type Vector) (a_dir :type Vector) (b_point :type Vector) (b_dir :type Vector))
  (bind (_x _y) (Math|Vector|BreakVector a_point))
  (bind (_x_2 _y_2) (Math|Vector|BreakVector b_point))
  (bind _returnvalue (+ b_point b_dir))
  (bind _returnvalue_2 (+ a_point a_dir))
  (bind (_x_3 _y_3) (Math|Vector|BreakVector _returnvalue_2))
  (bind (_x_4 _y_4) (Math|Vector|BreakVector _returnvalue))
  (LocalVariables|Setx1 _x)
  (LocalVariables|Sety1 _y)
  (LocalVariables|Setx2 _x_3)
  (LocalVariables|Sety2 _y_3)
  (LocalVariables|Setx3 _x_2)
  (LocalVariables|Sety3 _y_2)
  (LocalVariables|Setx4 _x_4)
  (LocalVariables|Sety4 _y_4)
  (bind _output_get (LocalVariables|Setdenominator (- (* (- (LocalVariables|Getx1) (LocalVariables|Getx2)) (- (LocalVariables|Gety3) (LocalVariables|Gety4))) (* (- (LocalVariables|Gety1) (LocalVariables|Gety2)) (- (LocalVariables|Getx3) (LocalVariables|Getx4))))))
  (LocalVariables|Sett (/ (- (* (- (LocalVariables|Getx1) (LocalVariables|Getx3)) (- (LocalVariables|Gety3) (LocalVariables|Gety4))) (* (- (LocalVariables|Gety1) (LocalVariables|Gety3)) (- (LocalVariables|Getx3) (LocalVariables|Getx4)))) (LocalVariables|Getdenominator)))
  (return (select (< (Math|Float|Absolute(Float) _output_get) 1e-05) a_point (Math|Vector|MakeVector (+ (LocalVariables|Getx1) (* (- (LocalVariables|Getx2) (LocalVariables|Getx1)) (LocalVariables|Gett))) (+ (LocalVariables|Gety1) (* (- (LocalVariables|Gety2) (LocalVariables|Gety1)) (LocalVariables|Gett))) 0.0)) (< (Math|Float|Absolute(Float) _output_get) 1e-05)))