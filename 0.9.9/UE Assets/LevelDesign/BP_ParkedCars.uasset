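; BP_ParkedCars is a level design actor that lines a spline with randomly chosen parked cars.
; Its construction script divides the spline length by Spacing (scaled by 100) and adds a skeletal mesh component from CarTypes at each step.
; Each car takes the spline's local location and rotation at a distance jittered by SpacingRandomness.
; The randomness uses no seed, and the event graph does nothing at runtime.
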(event EventBeginPlay)

(event Collision|EventActorBeginOverlap
  (params (OtherActor :type Actor%20Object%20Reference)))

(event EventTick
  (params (DeltaSeconds :type Float%20%28single-precision%29)))

(fn ConstructionScript
  (bind _car_types (Variables|Default|Getcar_types))
  (bind _spacing (Variables|Default|Getspacing))
  (bind _spline (Variables|Default|GetSpline))
  (bind _spacing_randomness (Variables|Default|Getspacing_randomness))
  (bind _returnvalue (* _spacing_randomness 1e+02))
  (bind _returnvalue_2 (* _spacing 1e+02))
  (for _index (range 0 (.ReturnValue (Math|Float|Division(WholeandRemainder) (Spline|GetSplineLength (Variables|Default|GetSpline)) _returnvalue_2)))
    (bind _returnvalue_3 (AddComponent|AddSkeletalMeshComponent false))
    (Class|SkinnedMeshComponent|SetSkeletalMesh _returnvalue_3 (Utilities|Array|Get(acopy) _car_types (Math|Random|RandomInteger (Utilities|Array|Length _car_types))) false)
    (Transformation|AddLocalOffset _returnvalue_3 (Spline|GetLocationatDistanceAlongSpline _spline (+ (* _index _returnvalue_2) (- (* (Math|Random|RandomFloat) _returnvalue) (/ _returnvalue 2.0))) "Local") false false)
    (Transformation|AddLocalRotation _returnvalue_3 (Spline|GetRotationatDistanceAlongSpline _spline (+ (* _index _returnvalue_2) (- (* (Math|Random|RandomFloat) _returnvalue) (/ _returnvalue 2.0))) "Local") false false)))