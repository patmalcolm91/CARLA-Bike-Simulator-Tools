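; Level design lane actor that extrudes a solid strip of set Width along its spline as a procedural mesh.
; The construction script builds one section per segment, with top and sides reaching down to BottomZ, plus a start endcap, with optional flat TopZ override.
; Corners are mitered by intersecting 2D offset lines between spline points, ignoring curvature.
; UVs are planar on top and follow accumulated edge length on the sides.
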(event EventBeginPlay)

(event Collision|EventActorBeginOverlap
  (params (OtherActor :type Actor%20Object%20Reference)))

(event EventTick
  (params (DeltaSeconds :type Float%20%28single-precision%29)))

(fn ConstructionScript
  (bind _returnvalue (Math|Float|MakeLiteralFloat 1.0))
  (bind _bottom_z (Variables|Default|Getbottom_z))
  (bind _material (Variables|Default|Getmaterial))
  (bind _width (Variables|Default|Getwidth))
  (bind _collision (Variables|Default|Getcollision))
  (bind _material_scale (Variables|Default|Getmaterial_scale))
  (bind _returnvalue_2 (* _material_scale 0.01))
  (bind _returnvalue_3 (* _width 1e+02))
  (bind _returnvalue_4 (Math|Float|MakeLiteralFloat _returnvalue_2))
  (bind _returnvalue_5 (AddComponent|AddProceduralMeshComponent false))
  (Variables|Default|Setmesh _returnvalue_5)
  (for _index (range 0 (Class|SplineComponent|GetNumberOfSplineSegments (Variables|Default|GetSpline)))
    (bind (_point_1 _point_2) (Utilities|GetCornersatSplinePoint _index)
      (:Exec_out
        (bind (_point_1_2 _point_2_2) (Utilities|GetCornersatSplinePoint (+ _index 1))
          (:Exec_out
            (Variables|Default|Sets_in_left (Variables|Default|Gets_out_left))
            (Variables|Default|Sets_out_left (+ (Variables|Default|Gets_out_left) (Math|Vector|Distance(Vector) (Utilities|DoZOverride _point_1) (Utilities|DoZOverride _point_1_2))))
            (Variables|Default|Sets_in_right (Variables|Default|Gets_out_right))
            (Variables|Default|Sets_out_right (+ (Variables|Default|Gets_out_right) (Math|Vector|Distance(Vector) (Utilities|DoZOverride _point_2) (Utilities|DoZOverride _point_2_2))))
            (if (== _index 0)
              (Class|ProceduralMeshComponent|CreateMeshSectionLinearColor (Variables|Default|Getmesh) 0 (Utilities|Array|MakeArray (Utilities|DoZOverride _point_1) (Math|Vector|MakeVector (.X (Math|Vector|BreakVector (Utilities|DoZOverride _point_1))) (.Y (Math|Vector|BreakVector (Utilities|DoZOverride _point_1))) _bottom_z) (Utilities|DoZOverride _point_2) (Math|Vector|MakeVector (.X (Math|Vector|BreakVector (Utilities|DoZOverride _point_2))) (.Y (Math|Vector|BreakVector (Utilities|DoZOverride _point_2))) _bottom_z)) (Variables|Default|Getendcap_triangle_indices) 0 (Utilities|Array|MakeArray "" (* (Math|Vector2D|MakeVector2D 0.0 (* (- (.Z (Math|Vector|BreakVector (Utilities|DoZOverride _point_1))) (Variables|Default|Getbottom_z)) _returnvalue)) _returnvalue_4) (* (Math|Vector2D|MakeVector2D _returnvalue_3 0.0) _returnvalue_4) (* (Math|Vector2D|MakeVector2D _returnvalue_3 (* (- (.Z (Math|Vector|BreakVector (Utilities|DoZOverride _point_1_2))) (Variables|Default|Getbottom_z)) _returnvalue)) _returnvalue_4)) 0 0 0 0 0 _collision)
              (Rendering|Material|SetMaterial (Variables|Default|Getmesh) 0 _material))
            (Class|ProceduralMeshComponent|CreateMeshSectionLinearColor (Variables|Default|Getmesh) (+ _index 1) (Utilities|Array|MakeArray (Utilities|DoZOverride _point_1) (Utilities|DoZOverride _point_2) (Utilities|DoZOverride _point_1_2) (Utilities|DoZOverride _point_2_2) (Utilities|DoZOverride _point_1) (Utilities|DoZOverride _point_2) (Utilities|DoZOverride _point_1_2) (Utilities|DoZOverride _point_2_2) (Math|Vector|MakeVector (.X (Math|Vector|BreakVector (Utilities|DoZOverride _point_1))) (.Y (Math|Vector|BreakVector (Utilities|DoZOverride _point_1))) _bottom_z) (Math|Vector|MakeVector (.X (Math|Vector|BreakVector (Utilities|DoZOverride _point_2))) (.Y (Math|Vector|BreakVector (Utilities|DoZOverride _point_2))) _bottom_z) (Math|Vector|MakeVector (.X (Math|Vector|BreakVector (Utilities|DoZOverride _point_1_2))) (.Y (Math|Vector|BreakVector (Utilities|DoZOverride _point_1_2))) _bottom_z) (Math|Vector|MakeVector (.X (Math|Vector|BreakVector (Utilities|DoZOverride _point_2_2))) (.Y (Math|Vector|BreakVector (Utilities|DoZOverride _point_2_2))) _bottom_z)) (Variables|Default|Gettriangle_indices) 0 (Utilities|Array|MakeArray (* (Math|Conversions|ToVector2D(Vector) (Utilities|DoZOverride _point_1)) _returnvalue_4) (* (Math|Conversions|ToVector2D(Vector) (Utilities|DoZOverride _point_2)) _returnvalue_4) (* (Math|Conversions|ToVector2D(Vector) (Utilities|DoZOverride _point_1_2)) _returnvalue_4) (* (Math|Conversions|ToVector2D(Vector) (Utilities|DoZOverride _point_2_2)) _returnvalue_4) (* (Math|Vector2D|MakeVector2D (Variables|Default|Gets_in_left) 0.0) _returnvalue_4) (* (Math|Vector2D|MakeVector2D (Variables|Default|Gets_in_right) 0.0) _returnvalue_4) (* (Math|Vector2D|MakeVector2D (Variables|Default|Gets_out_left) 0.0) _returnvalue_4) (* (Math|Vector2D|MakeVector2D (Variables|Default|Gets_out_right) 0.0) _returnvalue_4) (* (Math|Vector2D|MakeVector2D (Variables|Default|Gets_in_left) (* (- (.Z (Math|Vector|BreakVector (Utilities|DoZOverride _point_1))) (Variables|Default|Getbottom_z)) _returnvalue)) _returnvalue_4) (* (Math|Vector2D|MakeVector2D (Variables|Default|Gets_in_right) (* (- (.Z (Math|Vector|BreakVector (Utilities|DoZOverride _point_1))) (Variables|Default|Getbottom_z)) _returnvalue)) _returnvalue_4) (* (Math|Vector2D|MakeVector2D (Variables|Default|Gets_out_left) (* (- (.Z (Math|Vector|BreakVector (Utilities|DoZOverride _point_1_2))) (Variables|Default|Getbottom_z)) _returnvalue)) _returnvalue_4) (* (Math|Vector2D|MakeVector2D (Variables|Default|Gets_out_right) (* (- (.Z (Math|Vector|BreakVector (Utilities|DoZOverride _point_1_2))) (Variables|Default|Getbottom_z)) _returnvalue)) _returnvalue_4)) 0 0 0 0 0 _collision)
            (Rendering|Material|SetMaterial (Variables|Default|Getmesh) (+ _index 1) _material)))))))

(fn LineIntersection
  (params (a_point :type Vector) (a_dir :type Vector) (b_point :type Vector) (b_dir :type Vector))
  (bind (_x _y) (Math|Vector|BreakVector a_point))
  (bind (_x_2 _y_2) (Math|Vector|BreakVector b_point))
  (bind _returnvalue (+ b_point b_dir))
  (bind _returnvalue_2 (+ a_point a_dir))
  (bind (_x_3 _y_3) (Math|Vector|BreakVector _returnvalue_2))
  (bind (_x_4 _y_4) (Math|Vector|BreakVector _returnvalue))
  (LocalVariables|Setx1 _x)
  (LocalVariables|Sety1 _y)
  (LocalVariables|Setx2 _x_3)
  (LocalVariables|Sety2 _y_3)
  (LocalVariables|Setx3 _x_2)
  (LocalVariables|Sety3 _y_2)
  (LocalVariables|Setx4 _x_4)
  (LocalVariables|Sety4 _y_4)
  (bind _output_get (LocalVariables|Setdenominator (- (* (- (LocalVariables|Getx1) (LocalVariables|Getx2)) (- (LocalVariables|Gety3) (LocalVariables|Gety4))) (* (- (LocalVariables|Gety1) (LocalVariables|Gety2)) (- (LocalVariables|Getx3) (LocalVariables|Getx4))))))
  (LocalVariables|Sett (/ (- (* (- (LocalVariables|Getx1) (LocalVariables|Getx3)) (- (LocalVariables|Gety3) (LocalVariables|Gety4))) (* (- (LocalVariables|Gety1) (LocalVariables|Gety3)) (- (LocalVariables|Getx3) (LocalVariables|Getx4)))) (LocalVariables|Getdenominator)))
  (return (select (< (Math|Float|Absolute(Float) _output_get) 1e-05) a_point (Math|Vector|MakeVector (+ (LocalVariables|Getx1) (* (- (LocalVariables|Getx2) (LocalVariables|Getx1)) (LocalVariables|Gett))) (+ (LocalVariables|Gety1) (* (- (LocalVariables|Gety2) (LocalVariables|Gety1)) (LocalVariables|Gett))) 0.0)) (< (Math|Float|Absolute(Float) _output_get) 1e-05)))