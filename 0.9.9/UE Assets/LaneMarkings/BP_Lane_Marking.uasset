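; BP_Lane_Marking draws dashed lane markings along an editable spline.
; The Construction Script divides the spline length by dash-plus-spacing, converting metres to centimetres, and adds one spline mesh component per cycle.
; Each dash takes its endpoints and tangents from the spline, with lateral scale set from Width relative to a 0.1 base.
; The event graph holds no active logic.
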(event EventBeginPlay)

(event Collision|EventActorBeginOverlap
  (params (OtherActor :type Actor%20Object%20Reference)))

(event EventTick
  (params (DeltaSeconds :type Float%20%28single-precision%29)))

(fn ConstructionScript
  (bind _spline (Variables|Default|GetSpline))
  (bind _dash_length (Variables|Default|Getdash_length))
  (bind _width (Variables|Default|Getwidth))
  (bind _returnvalue (/ _width 0.1))
  (bind _returnvalue_2 (* _dash_length 1e+02))
  (bind _returnvalue_3 (Math|Vector2D|MakeVector2D _returnvalue 1.0))
  (bind _output_get (Variables|Default|Setcycle_length (+ _returnvalue_2 (* (Variables|Default|Getspacing) 1e+02))))
  (for _index (range 0 (.ReturnValue (Math|Float|Division(WholeandRemainder) (Spline|GetSplineLength (Variables|Default|GetSpline)) _output_get)))
    (bind _returnvalue_4 (AddComponent|AddSplineMeshComponent false))
    (Components|StaticMesh|SetStaticMesh _returnvalue_4 (Variables|Default|Getstatic_mesh))
    (SplineMesh|SetStartandEnd _returnvalue_4 (Spline|GetLocationatDistanceAlongSpline _spline (* (Math|Conversions|ToFloat(Integer) _index) (Variables|Default|Getcycle_length)) "Local") (Spline|GetTangentatDistanceAlongSpline _spline (* (Math|Conversions|ToFloat(Integer) _index) (Variables|Default|Getcycle_length)) "Local") (Spline|GetLocationatDistanceAlongSpline _spline (+ (* (Math|Conversions|ToFloat(Integer) _index) (Variables|Default|Getcycle_length)) _returnvalue_2) "Local") (Spline|GetTangentatDistanceAlongSpline _spline (+ (* (Math|Conversions|ToFloat(Integer) _index) (Variables|Default|Getcycle_length)) _returnvalue_2) "Local") true :!class /Script/Engine.SplineMeshComponent)
    (SplineMesh|SetStartScale _returnvalue_4 _returnvalue_3 true :!class /Script/Engine.SplineMeshComponent)
    (SplineMesh|SetEndScale _returnvalue_4 _returnvalue_3 true :!class /Script/Engine.SplineMeshComponent)))