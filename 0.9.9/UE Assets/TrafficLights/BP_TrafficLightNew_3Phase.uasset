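; Three-phase traffic light actor that shows red, yellow or green and relays state changes to car trigger observers.
; Construction script builds meshes from the Heads data, fits the pole to red-light height, and groups per-lamp dynamic materials by color, optionally masked.
; BeginPlay creates a trigger component for each box except TotalVolume.
; State changes toggle material On/Off parameters and notify those triggers; UnifyTriggers destroys all boxes except TotalVolume.
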(event Custom|Unify%20Triggers
  (for _array_element (Actor|GetComponentsByClass "/Script/Engine.BoxComponent")
    (if (not (Utilities|Enum|Equal(Enum) (Utilities|GetDisplayName _array_element) "TotalVolume"))
      (Components|DestroyComponent _array_element))))

(event EventBeginPlay
  (CallFunction|CreateCarObservers))

(event EventOnTrafficLightStateChanged
  (params (TrafficLightState :type ETrafficLightState%20Enum :default "Red"))
  (Utilities|FlowControl|Sequence
    (:then_0
      (switch Utilities|FlowControl|Switch|SwitchonETrafficLightState TrafficLightState
        (:Red
          (for _array_element (Variables|Default|GetRedLights)
            (Rendering|Material|SetScalarParameterValue _array_element "On/Off" 1.0 :!class /Script/Engine.MaterialInstanceDynamic))
          (for _array_element_2 (Variables|Default|GetYellowLights)
            (Rendering|Material|SetScalarParameterValue _array_element_2 "On/Off" 0.0 :!class /Script/Engine.MaterialInstanceDynamic))
          (for _array_element_3 (Variables|Default|GetGreenLights)
            (Rendering|Material|SetScalarParameterValue _array_element_3 "On/Off" 0.0 :!class /Script/Engine.MaterialInstanceDynamic)))
        (:Yellow
          (for _array_element_4 (Variables|Default|GetRedLights)
            (Rendering|Material|SetScalarParameterValue _array_element_4 "On/Off" 0.0 :!class /Script/Engine.MaterialInstanceDynamic))
          (for _array_element_5 (Variables|Default|GetYellowLights)
            (Rendering|Material|SetScalarParameterValue _array_element_5 "On/Off" 1.0 :!class /Script/Engine.MaterialInstanceDynamic))
          (for _array_element_6 (Variables|Default|GetGreenLights)
            (Rendering|Material|SetScalarParameterValue _array_element_6 "On/Off" 0.0 :!class /Script/Engine.MaterialInstanceDynamic)))
        (:Green
          (for _array_element_7 (Variables|Default|GetRedLights)
            (Rendering|Material|SetScalarParameterValue _array_element_7 "On/Off" 0.0 :!class /Script/Engine.MaterialInstanceDynamic))
          (for _array_element_8 (Variables|Default|GetYellowLights)
            (Rendering|Material|SetScalarParameterValue _array_element_8 "On/Off" 0.0 :!class /Script/Engine.MaterialInstanceDynamic))
          (for _array_element_9 (Variables|Default|GetGreenLights)
            (Rendering|Material|SetScalarParameterValue _array_element_9 "On/Off" 1.0 :!class /Script/Engine.MaterialInstanceDynamic)))))
    (:then_1
      (for _array_element_10 (Variables|Default|GetStoppedCarsMap)
        (Default|LightTrafficStateChanged _array_element_10 TrafficLightState)))))

(fn ConstructionScript
  (bind _cylinder (Variables|Default|GetCylinder))
  (bind _returnvalue (Transformation|GetWorldScale _cylinder))
  (bind (_x _y) (Math|Vector|BreakVector _returnvalue))
  (for _array_element (Variables|Default|GetHeads)
    (bind _returnvalue_2 (AddComponent|AddStaticMeshComponent false (Math|Conversions|ToTransform(Vector) (Math|Transform|TransformLocation (.Position (Utilities|Struct|BreakTrafficLightStructure _array_element)) (Math|Vector|MakeVector 0.0 0.0 (Variables|Default|Getheight_adjustment))))))
    (Components|StaticMesh|SetStaticMesh _returnvalue_2 "/Game/Carla/Static/TrafficSigns/Streetlights_01/SM_TL_BotCover.SM_TL_BotCover")
    (for _array_element_2 (.Lights (Utilities|Struct|BreakTrafficLightStructure _array_element))
      (bind _returnvalue_3 (AddComponent|AddStaticMeshComponent false (.RelativeTransform (Utilities|Struct|BreakTrafficLightPieceStructure _array_element_2))))
      (if (Utilities|Enum|Equal(Enum) (.LightColor (Utilities|Struct|BreakTrafficLightPieceStructure _array_element_2)) "NewEnumerator0")
        (Transformation|AddLocalOffset (Variables|Default|GetSM_TLights_Top) (Math|Vector|MakeVector 0.0 0.0 (.Z (Math|Vector|BreakVector (Math|Transform|TransformLocation (Math|Conversions|ToTransform(Vector) (Math|Transform|TransformLocation (.Position (Utilities|Struct|BreakTrafficLightStructure _array_element)) (Math|Vector|MakeVector 0.0 0.0 (Variables|Default|Getheight_adjustment)))) (Math|Transform|TransformLocation (.RelativeTransform (Utilities|Struct|BreakTrafficLightPieceStructure _array_element_2)) "0, 0,-56.000000"))))) false false)
        (Rendering|SetVisibility _cylinder (Variables|Default|Getshow_pole) false)
        (Transformation|SetRelativeScale3D _cylinder (Math|Vector|MakeVector _x _y (/ (.Z (Math|Vector|BreakVector (Math|Transform|TransformLocation (Math|Conversions|ToTransform(Vector) (Math|Transform|TransformLocation (.Position (Utilities|Struct|BreakTrafficLightStructure _array_element)) (Math|Vector|MakeVector 0.0 0.0 (Variables|Default|Getheight_adjustment)))) (Math|Transform|TransformLocation (.RelativeTransform (Utilities|Struct|BreakTrafficLightPieceStructure _array_element_2)) "0, 0,-56.000000")))) 1e+02)))
        (Transformation|AddLocalOffset _cylinder (Math|Vector|MakeVector 0.0 0.0 (/ (.Z (Math|Vector|BreakVector (Math|Transform|TransformLocation (Math|Conversions|ToTransform(Vector) (Math|Transform|TransformLocation (.Position (Utilities|Struct|BreakTrafficLightStructure _array_element)) (Math|Vector|MakeVector 0.0 0.0 (Variables|Default|Getheight_adjustment)))) (Math|Transform|TransformLocation (.RelativeTransform (Utilities|Struct|BreakTrafficLightPieceStructure _array_element_2)) "0, 0,-56.000000")))) 2.0)) false false))
      (Transformation|AttachComponentToComponent _returnvalue_3 _returnvalue_2 "None" "KeepRelative" "KeepRelative" "KeepRelative" false)
      (Components|StaticMesh|SetStaticMesh _returnvalue_3 (.Mesh (Utilities|Struct|BreakTrafficLightPieceStructure _array_element_2)))
      (if (Variables|Default|Getmasked)
        (bind _returnvalue_4 (Rendering|Material|CreateDynamicMaterialInstance _returnvalue_3 1 "/Game/Carla/Static/TrafficSigns/Streetlights_01/M_StreetlightsMasked.M_StreetlightsMasked" "None" :!class /Script/Engine.PrimitiveComponent))
        (LocalVariables|SetCurrentMaterial _returnvalue_4)
        (else
          (bind _returnvalue_5 (Rendering|Material|CreateDynamicMaterialInstance _returnvalue_3 1 "/Game/Carla/Static/TrafficSigns/Streetlights_01/M_StreetlightsMaster.M_StreetlightsMaster" "None" :!class /Script/Engine.PrimitiveComponent))
          (LocalVariables|SetCurrentMaterial _returnvalue_5)))
      (Rendering|Material|SetTextureParameterValue (LocalVariables|GetCurrentMaterial) "LightMask" (Variables|Default|GetMask))
      (Rendering|Material|SetScalarParameterValue (LocalVariables|GetCurrentMaterial) "Angle" (Variables|Default|Getmask_rotation) :!class /Script/Engine.MaterialInstanceDynamic)
      (switch Utilities|FlowControl|Switch|SwitchonStreetLightColor (.LightColor (Utilities|Struct|BreakTrafficLightPieceStructure _array_element_2))
        (:NewEnumerator0
          (Rendering|Material|SetVectorParameterValue (LocalVariables|GetCurrentMaterial) "LightColor" "(R=1.000000,G=0.015686,B=0.000000,A=1.000000)" :!class /Script/Engine.MaterialInstanceDynamic)
          (Utilities|Array|Add (Variables|Default|GetRedLights) (LocalVariables|GetCurrentMaterial)))
        (:NewEnumerator1
          (Rendering|Material|SetVectorParameterValue (LocalVariables|GetCurrentMaterial) "LightColor" "(R=1.000000,G=0.745098,B=0.000000,A=1.000000)" :!class /Script/Engine.MaterialInstanceDynamic)
          (Utilities|Array|Add (Variables|Default|GetYellowLights) (LocalVariables|GetCurrentMaterial)))
        (:NewEnumerator2
          (Rendering|Material|SetVectorParameterValue (LocalVariables|GetCurrentMaterial) "LightColor" "(R=0.000000,G=1.000000,B=0.000000,A=1.000000)" :!class /Script/Engine.MaterialInstanceDynamic)
          (Utilities|Array|Add (Variables|Default|GetGreenLights) (LocalVariables|GetCurrentMaterial)))))))

(fn GetTriggerVolume
  (return (Variables|Default|GetTotalVolume)))

(fn CreateCarObservers
  (for _array_element (Actor|GetComponentsByClass "/Script/Engine.BoxComponent")
    (if (not (Utilities|Enum|Equal(Enum) (Utilities|GetDisplayName _array_element) "TotalVolume"))
      (bind _returnvalue (AddComponent|AddBPCustomTriggerComponent))
      (Utilities|Array|Add (Variables|Default|GetStoppedCarsMap) _returnvalue)
      (Variables|/Game/Carla/Blueprints/TrafficLight/BP_CustomTriggerComponent.BP_CustomTriggerComponent_C|SetBoxCollider _returnvalue _array_element)
      (Default|BindOverlap _returnvalue))))